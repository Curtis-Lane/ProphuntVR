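; Game instance for the VR game that handles LAN multiplayer sessions for the Demonstration level.
; StartServer creates a four-slot session and opens the level as a listen server, while FindServers searches and passes the first result to JoinServer.
; StartGame server-travels to the same level, and failures only print messages.
; An unused find-or-host chain with retry delays remains in the graph but never runs.
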(event `StartServer`
  (`CreateSessionCallbackProxy.CreateSession` (`GameplayStatics.GetPlayerController` 0) 4 true false
    (:`OnSuccess`
      (`GameplayStatics.OpenLevelBySoftObjectPtr` "/Game/PolygonOffice/Maps/Demonstration.Demonstration" true "listen"))
    (:`OnFailure`
      (`KismetSystemLibrary.PrintString` "Failed To Create Session"))))

(event `JoinServer`
  (params (SessionResult :type "BlueprintSessionResult Structure"))
  (`JoinSessionCallbackProxy.JoinSession` (`GameplayStatics.GetPlayerController` 0) SessionResult
    (:`OnFailure`
      (`KismetSystemLibrary.PrintString` "Failed To Join Session"))))

(event `FindServers`
  (bind _results (`FindSessionsCallbackProxy.FindSessions` (`GameplayStatics.GetPlayerController` 0) 0 true)
    (:`OnSuccess`
      (if (!= (`KismetArrayLibrary.Array_Length` _results) 0)
        (`self.JoinServer` (`|GetArrayItem` _results))
        (else
          (`KismetSystemLibrary.PrintString` "Found Zero Sessions"))))
    (:`OnFailure`
      (`KismetSystemLibrary.PrintString` "Failed To Find Sessions"))))

(event `StartGame`
  (`KismetSystemLibrary.ExecuteConsoleCommand` "servertravel Demonstration" (`GameplayStatics.GetPlayerController` 0)))